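; BP_Enemy is a simple enemy actor that announces itself on BeginPlay and takes damage through a HealthDamage event.
; HealthDamage subtracts incoming damage from Health and prints the new value to the screen.
; An AliveCheck function treats Health above a small threshold as alive; otherwise the enemy prints a death message and destroys itself after a short delay.
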(event Custom|HealthDamage
  (params (Incoming%20Damage :type Float%20%28double-precision%29))
  (Variables|Default|SetHealth (- (Variables|Default|GetHealth) Incoming%20Damage))
  (Development|PrintString (Utilities|String|Append "Ouch! my health is Now: " (Utilities|String|ToString(Float) (Variables|Default|GetHealth))) true true "(R=0.000000,G=0.660000,B=1.000000,A=1.000000)" 5.0)
  (if (CallFunction|AliveCheck (Variables|Default|GetHealth))
    (Development|PrintString "Still Alive!" true true "(R=0.000000,G=0.660000,B=1.000000,A=1.000000)" 5.0)
    (else
      (Development|PrintString "Ded" true true "(R=0.000000,G=0.660000,B=1.000000,A=1.000000)" 5.0)
      (Utilities|FlowControl|Delay 1.0)
      (Actor|DestroyActor))))

(event EventBeginPlay
  (Development|PrintString "I am going to destroy you!"))

(fn ConstructionScript)

(fn AliveCheck
  (params (Incoming%20Health :type Float%20%28double-precision%29))
  (return (> Incoming%20Health 0.5)))