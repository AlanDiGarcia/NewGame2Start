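; BP_Launcher is an item that fires BP_Bullet projectiles from a limited ammo pool.
; UsePrimary, while ammo remains, spawns a bullet at the SpawnPoint location, calls its Shoot with the forward vector scaled by ShootForce, and decrements Ammo.
; ReplenishAmmo adds incoming ammo to the count without a cap, and the current count is printed on begin play and after each change.
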(event Custom|Replenish%20Ammo
  (params (Incoming%20Ammo :type Integer))
  (Variables|Default|SetAmmo (+ Incoming%20Ammo (Variables|Default|GetAmmo)))
  (Development|PrintString (Utilities|String|Append "Ammo: " (Utilities|String|ToString(Integer) (Variables|Default|GetAmmo)))))

(event EventBeginPlay
  (Development|PrintString (Utilities|String|Append "Ammo: " (Utilities|String|ToString(Integer) (Variables|Default|GetAmmo)))))

(event EventUsePrimary
  (if (> (Variables|Default|GetAmmo) 0)
    (bind _returnvalue (Game|SpawnActorfromClass "/Game/Items/BP_Bullet.BP_Bullet_C" (Math|Transform|MakeTransform (Transformation|GetWorldLocation (Variables|Default|GetSpawn%20Point)) "0, 0, 0" "1.000000,1.000000,1.000000") "Undefined" "MultiplyWithRoot" 0 0))
    (Default|Shoot _returnvalue (* (Math|Vector|GetForwardVector (Variables|Default|GetSpawn%20Point)) (Variables|Default|GetShoot%20Force)))
    (Math|Integer|DecrementInt (Variables|Default|GetAmmo)
      (:%20%20
        (Development|PrintString (Utilities|String|Append "Ammo: " (Utilities|String|ToString(Integer) (Variables|Default|GetAmmo))))))))

(fn ConstructionScript
  (|CallParentFunction))