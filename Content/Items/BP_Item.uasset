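; BP_Item is a physics item actor that can be picked up into a hand and dropped or thrown.
; ItemPickup disables physics and collision on the Cube component, then snaps it to the hand_r_sok socket of the incoming mesh.
; ItemDrop detaches the Cube in world space, restores collision and physics, and applies the supplied force as an impulse.
; UsePrimary is an empty event with no behavior in this Blueprint.
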(event Custom|ItemPickup
  (params (Incoming%20Mesh :type Scene%20Component%20Object%20Reference))
  (Physics|SetSimulatePhysics (Variables|Default|GetCube) false)
  (Collision|SetCollisionEnabled (Variables|Default|GetCube) "NoCollision")
  (Transformation|AttachComponentToComponent (Variables|Default|GetCube) Incoming%20Mesh "hand_r_sok" "SnapToTarget" "SnapToTarget" "KeepRelative" true))

(event Custom|ItemDrop
  (params (Incoming%20Force :type Vector))
  (Transformation|DetachFromComponent (Variables|Default|GetCube) "KeepWorld" "KeepWorld" "KeepRelative" true)
  (Collision|SetCollisionEnabled (Variables|Default|GetCube) "QueryAndPhysics")
  (Physics|SetSimulatePhysics (Variables|Default|GetCube) true)
  (Physics|AddImpulse (Variables|Default|GetCube) Incoming%20Force "None" false))

(event Custom|Use%20Primary)

(fn ConstructionScript)