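; Spawner that runs an escalating, timed knock-ball minigame, scattering BP_KnockBall actors at random XY offsets around itself.
; ActivateKnocking either spawns a wave and starts a timer shared with BP_TimerKnock, or ends the game, resetting difficulty and destroying balls.
; On timeout, any remaining ball respawns the player; otherwise the next wave starts with more balls and a longer timer.
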(event Custom|Check%20KnockBalls
  (Math|Integer|IncrementInt (Variables|Default|GetNumBalls)
    (:%20%20
      (Math|Integer|IncrementInt (Variables|Default|GetNumBalls)
        (:%20%20
          (bind _outactors (Actor|GetAllActorsOfClass "/Game/PersonalProject/BP_KnockBall.BP_KnockBall_C"))
          (if (!= (Utilities|Array|Length _outactors) 0)
            (bind _returnvalue (Actor|GetActorOfClass "/Game/ThirdPerson/Blueprints/BP_ThirdPersonCharacter.BP_ThirdPersonCharacter_C"))
            (Default|RespawnPlayer _returnvalue)
            (else
              (Variables|Default|SetDuration (+ (Variables|Default|GetDuration) 1.0))
              (CallFunction|ResetLoop))))))))

(event Custom|Game%20End
  (Variables|Default|SetDuration 12.0)
  (Variables|Default|SetNumBalls 3)
  (bind _outactors (Actor|GetAllActorsOfClass "/Game/PersonalProject/BP_KnockBall.BP_KnockBall_C"))
  (for _array_element _outactors
    (Actor|DestroyActor _array_element)))

(event Custom|Spawn%20Knockballs
  (bind _returnvalue (Transformation|GetActorLocation))
  (for _index (range 1 (Variables|Default|GetNumBalls))
    (Game|SpawnActorfromClass "/Game/PersonalProject/BP_KnockBall.BP_KnockBall_C" (Math|Transform|MakeTransform (Math|Vector|MakeVector (+ (Math|Random|RandomFloatinRange -2e+03 2e+03) (.x _returnvalue)) (+ (Math|Random|RandomFloatinRange -2e+03 2e+03) (.y _returnvalue)) (.z _returnvalue)) "0, 0, 0" "1.000000,1.000000,1.000000") "AdjustIfPossibleButAlwaysSpawn" "MultiplyWithRoot" 0 0)))

(event Custom|Activate%20Time
  (bind _returnvalue (Utilities|Time|SetTimerbyEvent (delegate Custom|Check%20KnockBalls) (Variables|Default|GetDuration)))
  (Variables|Default|SetTime%20Handle _returnvalue)
  (bind _returnvalue_2 (Actor|GetActorOfClass "/Game/PersonalProject/BP_TimerKnock.BP_TimerKnock_C"))
  (Default|Timing _returnvalue_2 (Variables|Default|GetTime%20Handle)))

(event Custom|Reset%20Loop
  (if (stale EventActivateKnocking Incoming%20Knocking)
    (CallFunction|SpawnKnockballs)
    (CallFunction|ActivateTime)
    (else
      (CallFunction|GameEnd))))

(event EventActivateKnocking
  (params (Incoming%20Knocking :type Boolean))
  (if Incoming%20Knocking
    (CallFunction|SpawnKnockballs)
    (CallFunction|ActivateTime)
    (else
      (CallFunction|GameEnd))))

(event EventBeginPlay)

(fn ConstructionScript)