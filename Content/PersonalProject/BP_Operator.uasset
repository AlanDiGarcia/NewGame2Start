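; BP_Operator is a trigger that launches one of four minigames: dancing, shooting, dodging or knocking.
; Selector stores the chosen game and updates the BP_OperatorText display.
; When the third-person character overlaps its box, it teleports them via the matching spawn point, waits briefly, then activates that game's actors, found by class lookup.
; EndGames deactivates whichever game is currently selected.
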(event OnComponentBeginOverlap(Box)
  (params (OverlappedComponent :type Primitive%20Component%20Object%20Reference) (OtherActor :type Actor%20Object%20Reference) (OtherComp :type Primitive%20Component%20Object%20Reference) (OtherBodyIndex :type Integer) (bFromSweep :type Boolean) (SweepResult :type Hit%20Result%20Structure%20%28by%20ref%29))
  (Utilities|Casting|CastToBP_ThirdPersonCharacter OtherActor)
  (switch int (Variables|Default|GetSelection)
    (:0
      (Variables|Default|SetDancing true)
      (bind _returnvalue (Actor|GetActorOfClass "/Game/PersonalProject/BP_SpawnPointDance.BP_SpawnPointDance_C"))
      (Default|TeleportPlayer _returnvalue)
      (Utilities|FlowControl|Delay 1.0)
      (bind _outactors (Actor|GetAllActorsOfClass "/Game/PersonalProject/BP_DancePlatform.BP_DancePlatform_C"))
      (bind _array_element (Utilities|Array|ForEachLoopwithBreak _outactors)
        (:LoopBody
          (Default|ActivateDancing _array_element (Variables|Default|GetDancing)))))
    (:1
      (Variables|Default|SetShooting true)
      (bind _returnvalue_2 (Actor|GetActorOfClass "/Game/PersonalProject/BP_SpawnPointShoot.BP_SpawnPointShoot_C"))
      (Default|TeleportPlayer _returnvalue_2)
      (Utilities|FlowControl|Delay 1.0)
      (bind _returnvalue_3 (Actor|GetActorOfClass "/Game/PersonalProject/BP_ShootTargetOperator.BP_ShootTargetOperator_C"))
      (Default|ActivateShooting _returnvalue_3 (Variables|Default|GetShooting)))
    (:2
      (Variables|Default|SetDodging true)
      (bind _returnvalue_4 (Actor|GetActorOfClass "/Game/PersonalProject/BP_SpawnPointDodge.BP_SpawnPointDodge_C"))
      (Default|TeleportPlayer _returnvalue_4)
      (Utilities|FlowControl|Delay 1.0)
      (bind _returnvalue_5 (Actor|GetActorOfClass "/Game/PersonalProject/BP_DodgeBallSpawner.BP_DodgeBallSpawner_C"))
      (Default|ActivateDodging _returnvalue_5 (Variables|Default|GetDodging)))
    (:3
      (Variables|Default|SetKnocking true)
      (bind _returnvalue_6 (Actor|GetActorOfClass "/Game/PersonalProject/BP_SpawnPointKnocking.BP_SpawnPointKnocking_C"))
      (Default|TeleportPlayer _returnvalue_6)
      (Utilities|FlowControl|Delay 1.0)
      (bind _returnvalue_7 (Actor|GetActorOfClass "/Game/PersonalProject/BP_KnockBallSpawner.BP_KnockBallSpawner_C"))
      (Default|ActivateKnocking _returnvalue_7 (Variables|Default|GetKnocking)))))

(event Custom|End%20Games
  (switch int (Variables|Default|GetSelection)
    (:0
      (Variables|Default|SetDancing false)
      (bind _outactors (Actor|GetAllActorsOfClass "/Game/PersonalProject/BP_DancePlatform.BP_DancePlatform_C"))
      (bind _array_element (Utilities|Array|ForEachLoopwithBreak _outactors)
        (:LoopBody
          (Default|ActivateDancing _array_element (Variables|Default|GetDancing)))))
    (:1
      (Variables|Default|SetShooting false)
      (bind _returnvalue (Actor|GetActorOfClass "/Game/PersonalProject/BP_ShootTargetOperator.BP_ShootTargetOperator_C"))
      (Default|ActivateShooting _returnvalue (Variables|Default|GetShooting)))
    (:2
      (Variables|Default|SetDodging false)
      (bind _returnvalue_2 (Actor|GetActorOfClass "/Game/PersonalProject/BP_DodgeBallSpawner.BP_DodgeBallSpawner_C"))
      (Default|ActivateDodging _returnvalue_2 (Variables|Default|GetDodging)))
    (:3
      (Variables|Default|SetKnocking false)
      (bind _returnvalue_3 (Actor|GetActorOfClass "/Game/PersonalProject/BP_KnockBallSpawner.BP_KnockBallSpawner_C"))
      (Default|ActivateKnocking _returnvalue_3 (Variables|Default|GetKnocking)))))

(event EventSelector
  (params (Incoming%20Selection :type Integer))
  (Variables|Default|SetSelection Incoming%20Selection)
  (bind _returnvalue (Actor|GetActorOfClass "/Game/PersonalProject/BP_OperatorText.BP_OperatorText_C"))
  (Default|TextChange _returnvalue (Variables|Default|GetSelection)))

(fn ConstructionScript)