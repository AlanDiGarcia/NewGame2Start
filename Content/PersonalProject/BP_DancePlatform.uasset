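; BP_DancePlatform is a dance-floor tile that randomly turns deadly in timed rounds while dancing is active.
; Each round a weighted roll picks teal or warning yellow, with yellow turning red and spawning a BP_KillBoxDance.
; A timer ends the round, raises the danger weight, destroys every kill box in the level and loops.
; Deactivation resets weight and material and clears the kill boxes.
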(event Custom|Deadly
  (Rendering|Material|SetMaterial (Variables|Default|GetCube) 0 "/Game/Materials/MI_FlatRed.MI_FlatRed")
  (Game|SpawnActorfromClass "/Game/PersonalProject/BP_KillBoxDance.BP_KillBoxDance_C" (Math|Transform|MakeTransform (Transformation|GetActorLocation) "0, 0, 0" "7.000000,7.000000,4.000000") "Undefined" "MultiplyWithRoot" 0 0))

(event Custom|Round%20End
  (Variables|Default|SetWeight (+ (Variables|Default|GetWeight) 0.05))
  (bind _outactors (Actor|GetAllActorsOfClass "/Game/PersonalProject/BP_KillBoxDance.BP_KillBoxDance_C"))
  (for _array_element _outactors
    (Actor|DestroyActor _array_element))
  (CallFunction|ResetLoop))

(event Custom|Tile%20Outcome
  (if (Math|Random|RandomBoolwithWeight (Variables|Default|GetWeight))
    (Rendering|Material|SetMaterial (Variables|Default|GetCube) 0 "/Game/Materials/MI_FlatYellow.MI_FlatYellow")
    (Utilities|Time|SetTimerbyEvent (delegate Custom|Deadly) 1.5)
    (else
      (Rendering|Material|SetMaterial (Variables|Default|GetCube) 0 "/Game/Materials/MI_FlatTeal.MI_FlatTeal")))
  (Utilities|Time|SetTimerbyEvent (delegate Custom|Round%20End) 3.5))

(event Custom|Game%20End
  (Variables|Default|SetWeight 0.05)
  (Rendering|Material|SetMaterial (Variables|Default|GetCube) 0 "/Game/Footsteps/MI_Default.MI_Default")
  (bind _outactors (Actor|GetAllActorsOfClass "/Game/PersonalProject/BP_KillBoxDance.BP_KillBoxDance_C"))
  (for _array_element _outactors
    (Actor|DestroyActor _array_element)))

(event Custom|Reset%20Loop
  (if (stale EventActivateDancing Incoming%20Dancing)
    (CallFunction|TileOutcome)
    (else
      (CallFunction|GameEnd))))

(event EventActivateDancing
  (params (Incoming%20Dancing :type Boolean))
  (if Incoming%20Dancing
    (CallFunction|TileOutcome)
    (else
      (CallFunction|GameEnd))))

(fn ConstructionScript)