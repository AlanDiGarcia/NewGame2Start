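; BP_ShootTarget is a shooting target that can be randomly armed and then knocked out by a bullet.
; ActivateTargeting rolls a weighted random chance and, on success, marks the target active and turns its cylinder yellow.
; When a BP_Bullet overlaps the sphere of an active target, matched by class display name, it destroys the bullet and restores the default material.
; A scoreboard scoring call exists but is disconnected, so hits award no points here.
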(event OnComponentBeginOverlap(Sphere)
  (params (OverlappedComponent :type Primitive%20Component%20Object%20Reference) (OtherActor :type Actor%20Object%20Reference) (OtherComp :type Primitive%20Component%20Object%20Reference) (OtherBodyIndex :type Integer) (bFromSweep :type Boolean) (SweepResult :type Hit%20Result%20Structure%20%28by%20ref%29))
  (if (and (Utilities|Enum|Equal(Enum) (Utilities|GetClassDisplayName (Utilities|GetClass OtherActor)) "BP_Bullet_C") (Variables|Default|GetActivated%20Target))
    (Actor|DestroyActor OtherActor)
    (Variables|Default|SetActivated%20Target false)
    (Rendering|Material|SetMaterial (Variables|Default|GetCylinder) 0 "/Game/Footsteps/MI_Default.MI_Default")))

(event Custom|Target%20Activation
  (Variables|Default|SetActivated%20Target true)
  (Rendering|Material|SetMaterial (Variables|Default|GetCylinder) 0 "/Game/Materials/MI_FlatYellow.MI_FlatYellow"))

(event EventActivateTargeting
  (params (Incoming%20Weight :type Float%20%28double-precision%29))
  (if (Math|Random|RandomBoolwithWeight Incoming%20Weight)
    (CallFunction|TargetActivation)))

(fn ConstructionScript)