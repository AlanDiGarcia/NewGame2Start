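; BP_ShootTargetOperator runs a timed shooting-target challenge across all BP_ShootTarget actors.
; While IncomingShooting is set, each round activates targets using Weight, starts a timer and passes its handle to BP_TimerTarget.
; At round end, any still-active target respawns the player, then the loop restarts and Weight rises.
; When shooting is off, it resets Weight, Duration and every target's state and material.
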(event Custom|Round%20End
  (bind _outactors (Actor|GetAllActorsOfClass "/Game/PersonalProject/BP_ShootTarget.BP_ShootTarget_C"))
  (bind _array_element (Utilities|Array|ForEachLoopwithBreak _outactors :!label _label)
    (:LoopBody
      (if (Variables|/Game/PersonalProject/BP_ShootTarget.BP_ShootTarget_C|GetActivated%20Target _array_element)
        (bind _returnvalue (Actor|GetActorOfClass "/Game/ThirdPerson/Blueprints/BP_ThirdPersonCharacter.BP_ThirdPersonCharacter_C"))
        (Default|RespawnPlayer _returnvalue)
        (goto _label Break)))
    (:Completed
      (CallFunction|ResetLoop)
      (Variables|Default|SetWeight (+ (Variables|Default|GetWeight) 0.05)))))

(event Custom|Game%20End
  (Variables|Default|SetWeight 0.15)
  (Variables|Default|SetDuration 7.0)
  (bind _outactors (Actor|GetAllActorsOfClass "/Game/PersonalProject/BP_ShootTarget.BP_ShootTarget_C"))
  (for _array_element _outactors
    (Variables|/Game/PersonalProject/BP_ShootTarget.BP_ShootTarget_C|SetActivated%20Target _array_element false)
    (Rendering|Material|SetMaterial (Variables|/Game/PersonalProject/BP_ShootTarget.BP_ShootTarget_C|GetCylinder _array_element) 0 "/Game/Footsteps/MI_Default.MI_Default")))

(event Custom|Target%20Activation
  (bind _outactors (Actor|GetAllActorsOfClass "/Game/PersonalProject/BP_ShootTarget.BP_ShootTarget_C"))
  (for _array_element _outactors
    (Default|ActivateTargeting _array_element (Variables|Default|GetWeight))))

(event Custom|Reset%20Loop
  (if (stale EventActivateShooting Incoming%20Shooting)
    (CallFunction|TargetActivation)
    (CallFunction|ActivateTime)
    (else
      (CallFunction|GameEnd))))

(event Custom|Activate%20Time
  (bind _returnvalue (Utilities|Time|SetTimerbyEvent (delegate Custom|Round%20End) (Variables|Default|GetDuration)))
  (Variables|Default|SetTime%20Handle _returnvalue)
  (bind _returnvalue_2 (Actor|GetActorOfClass "/Game/PersonalProject/BP_TimerTarget.BP_TimerTarget_C"))
  (Default|Timing _returnvalue_2 (Variables|Default|GetTime%20Handle)))

(event EventActivateShooting
  (params (Incoming%20Shooting :type Boolean))
  (if Incoming%20Shooting
    (CallFunction|TargetActivation)
    (CallFunction|ActivateTime)
    (else
      (CallFunction|GameEnd))))

(fn ConstructionScript)