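; Moving shooting target that slides a Cylinder between the Start and End component positions.
; On BeginPlay it seeks a Timeline to a random time between 0 and 1, then plays it, so instances can start out of step.
; Each Timeline update lerps the Cylinder's world location using the track value as alpha, without sweep.
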(event EventBeginPlay
  (Utilities|FlowControl|Sequence
    (:then_0
      (bind _newtrack_0 (Timeline|Timeline SetNewTime)
        (:Update
          (Transformation|SetWorldLocation (Variables|Default|GetCylinder) (Math|Vector|Lerp(Vector) (Transformation|GetWorldLocation (Variables|Default|GetStart)) (Transformation|GetWorldLocation (Variables|Default|GetEnd)) _newtrack_0) false false))))
    (:then_1
      (Timeline|Timeline Play))))

(fn ConstructionScript
  (|CallParentFunction))