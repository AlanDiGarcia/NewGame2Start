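; BP_DodgeBall is a hazard ball that homes in on the player character and respawns them on contact.
; It enables Tick after a short delay on BeginPlay.
; Each tick looks up the third-person character and moves the Sphere component toward its capsule at constant speed, with sweep enabled.
; An overlap on a second component, Sphere1, casts to that character and calls RespawnPlayer.
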(event OnComponentBeginOverlap(Sphere1)
  (params (OverlappedComponent :type Primitive%20Component%20Object%20Reference) (OtherActor :type Actor%20Object%20Reference) (OtherComp :type Primitive%20Component%20Object%20Reference) (OtherBodyIndex :type Integer) (bFromSweep :type Boolean) (SweepResult :type Hit%20Result%20Structure%20%28by%20ref%29))
  (bind _asbp_third_person_character (Utilities|Casting|CastToBP_ThirdPersonCharacter OtherActor))
  (Default|RespawnPlayer _asbp_third_person_character))

(event EventTick
  (params (DeltaSeconds :type Float%20%28single-precision%29))
  (bind _returnvalue (Actor|GetActorOfClass "/Game/ThirdPerson/Blueprints/BP_ThirdPersonCharacter.BP_ThirdPersonCharacter_C"))
  (Transformation|SetWorldLocation (Variables|Default|GetSphere) (Math|Interpolation|VInterptoConstant (Transformation|GetWorldLocation (Variables|Default|GetSphere)) (Transformation|GetWorldLocation (Variables|/Script/Engine.Character|GetCapsuleComponent _returnvalue)) DeltaSeconds 7e+02) true false))

(event EventBeginPlay
  (Utilities|FlowControl|Delay 2.5)
  (Actor|Tick|SetActorTickEnabled true))

(fn ConstructionScript)