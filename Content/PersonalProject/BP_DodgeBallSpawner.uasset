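; Dodgeball spawner actor that drops BP_DodgeBall actors at random X/Y points within a square around itself, at its own height.
; ActivateDodging either starts the spawn loop or ends the game, depending on its IncomingDodging flag.
; Each spawn sets a one-shot timer to LessTime, which shortens the delay down to a floor and loops back, so spawns speed up.
; GameEnd resets the delay and destroys all dodgeballs.
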(event Custom|Less%20Time
  (Variables|Default|SetDuration (- (Variables|Default|GetDuration) 0.3))
  (if (<= (Variables|Default|GetDuration) 1.2)
    (Variables|Default|SetDuration 1.2))
  (CallFunction|ResetLoop))

(event Custom|Game%20End
  (Variables|Default|SetDuration 4.5)
  (bind _outactors (Actor|GetAllActorsOfClass "/Game/PersonalProject/BP_DodgeBall.BP_DodgeBall_C"))
  (for _array_element _outactors
    (Actor|DestroyActor _array_element)))

(event Custom|Spawn%20Dodgeballs
  (bind _returnvalue (Transformation|GetActorLocation))
  (Game|SpawnActorfromClass "/Game/PersonalProject/BP_DodgeBall.BP_DodgeBall_C" (Math|Transform|MakeTransform (Math|Vector|MakeVector (+ (Math|Random|RandomFloatinRange -2e+03 2e+03) (.x _returnvalue)) (+ (Math|Random|RandomFloatinRange -2e+03 2e+03) (.y _returnvalue)) (.z _returnvalue)) "0, 0, 0" "1.000000,1.000000,1.000000") "AdjustIfPossibleButAlwaysSpawn" "MultiplyWithRoot" 0 0)
  (Utilities|Time|SetTimerbyEvent (delegate Custom|Less%20Time) (Variables|Default|GetDuration)))

(event Custom|Reset%20Loop
  (if (stale EventActivateDodging Incoming%20Dodging)
    (CallFunction|SpawnDodgeballs)
    (else
      (CallFunction|GameEnd))))

(event EventBeginPlay)

(event EventActivateDodging
  (params (Incoming%20Dodging :type Boolean))
  (if Incoming%20Dodging
    (CallFunction|SpawnDodgeballs)
    (else
      (CallFunction|GameEnd))))

(fn ConstructionScript)