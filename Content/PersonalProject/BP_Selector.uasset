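; BP_Selector is a trigger actor that steps through a selection index whenever the third-person character enters its box.
; Each overlap increments Selection and passes it to the Selector function on the BP_Operator found with GetActorOfClass.
; Once Selection reaches three, it resets to minus one after sending, so the next overlap wraps the cycle back to zero.
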(event OnComponentBeginOverlap(Box)
  (params (OverlappedComponent :type Primitive%20Component%20Object%20Reference) (OtherActor :type Actor%20Object%20Reference) (OtherComp :type Primitive%20Component%20Object%20Reference) (OtherBodyIndex :type Integer) (bFromSweep :type Boolean) (SweepResult :type Hit%20Result%20Structure%20%28by%20ref%29))
  (Utilities|Casting|CastToBP_ThirdPersonCharacter OtherActor)
  (CallFunction|SelectionProcess))

(event Custom|Send%20Selection
  (bind _returnvalue (Actor|GetActorOfClass "/Game/PersonalProject/BP_Operator.BP_Operator_C"))
  (Default|Selector _returnvalue (Variables|Default|GetSelection)))

(event Custom|Selection%20Process
  (Math|Integer|IncrementInt (Variables|Default|GetSelection)
    (:%20%20
      (CallFunction|SendSelection)
      (if (>= (Variables|Default|GetSelection) 3)
        (Variables|Default|SetSelection -1)))))

(fn ConstructionScript)