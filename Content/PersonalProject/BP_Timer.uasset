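; BP_Timer is an in-world countdown display that shows a timer's remaining time on four text render components.
; Its Timing event receives and stores a timer handle from outside, so the Blueprint only displays a timer it does not start itself.
; Every Tick it queries that handle's remaining time, replaces non-positive values with zero, and writes the result to all four texts.
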(event EventTick
  (params (DeltaSeconds :type Float%20%28single-precision%29))
  (Variables|Default|SetTime (Utilities|Time|GetTimerRemainingTimebyHandle (Variables|Default|GetTime%20Handle)))
  (if (> (Variables|Default|GetTime) 0.0)
    _
    (else
      (Variables|Default|SetTime 0.0)))
  (Rendering|Components|TextRender|SetText (Variables|Default|GetTextRender) (Utilities|Text|ToText(Float) (Variables|Default|GetTime) "HalfToEven" false true 1 324 0 1))
  (Rendering|Components|TextRender|SetText (Variables|Default|GetTextRender1) (Utilities|Text|ToText(Float) (Variables|Default|GetTime) "HalfToEven" false true 1 324 0 1))
  (Rendering|Components|TextRender|SetText (Variables|Default|GetTextRender2) (Utilities|Text|ToText(Float) (Variables|Default|GetTime) "HalfToEven" false true 1 324 0 1))
  (Rendering|Components|TextRender|SetText (Variables|Default|GetTextRender3) (Utilities|Text|ToText(Float) (Variables|Default|GetTime) "HalfToEven" false true 1 324 0 1)))

(event EventTiming
  (params (Incoming%20Time%20Handle :type Timer%20Handle%20Structure))
  (Variables|Default|SetTime%20Handle Incoming%20Time%20Handle))

(fn ConstructionScript)